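; Bonfire actor that acts as an interactable save point in the ActionRougue game.
; Interact sets FireActive, calls WriteSaveGame on PGameModeBase, prints a confirmation and updates the flames.
; UpdateFlames activates the particle system when FireActive is set, and OnActorLoaded calls it again to refresh the visual after loading.
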(event Custom|UpdateFlames
  (if (Variables|Default|GetbFireActive)
    (Components|Activation|Activate (Variables|Default|GetParticleSystem) false)))

(event EventBeginPlay)

(event Collision|EventActorBeginOverlap
  (params (OtherActor :type Actor%20Object%20Reference)))

(event EventTick
  (params (DeltaSeconds :type Float%20%28single-precision%29)))

(event EventInteract
  (params (InstigatorPawn :type Pawn%20Object%20Reference))
  (Variables|Default|SetbFireActive true)
  (bind _aspgame_mode_base (Utilities|Casting|CastToPGameModeBase (Game|GetGameMode)))
  (Class|PGameModeBase|WriteSaveGame _aspgame_mode_base)
  (Development|PrintString "WORLD SAVED")
  (CallFunction|UpdateFlames))

(event EventOnActorLoaded
  (CallFunction|UpdateFlames))

(fn ConstructionScript)